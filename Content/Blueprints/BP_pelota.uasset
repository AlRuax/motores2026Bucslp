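; BP_pelota is an actor, named as a ball, that destroys itself after a set lifetime.
; Tick accumulates delta time in Incremento and destroys the actor once it reaches TiempoVida.
; BeginPlay also adds a fixed amount to Vida, which nothing else in these graphs reads.
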(event `self.ReceiveBeginPlay`
  (set `self.vida` (+ (`self.vida`) 10.0)))

(event `self.ReceiveTick`
  (params (DeltaSeconds :type "Float (single-precision)"))
  (bind _output_get (set `self.incremento` (+ DeltaSeconds (`self.incremento`))))
  (if (>= _output_get (`self.TiempoVida`))
    (`self.K2_DestroyActor`)))

(fn `UserConstructionScript`)